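; Player character that uses the Gameplay Ability System for size-changing classes: Pixie, Titan and Versatile.
; BeginPlay grants default stats, stamina regen and melee, then class abilities and effects chosen by the game instance's SelectedClass, all targeting player character 0.
; Enhanced Input events activate transform, dash and melee abilities by class.
; M_SmoothResize uses a timeline to lerp uniform actor scale from the mesh's relative X scale to a target.
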(event Custom|M_SmoothResize
  (params (TargetScale :type Float%20%28double-precision%29))
  ;[0.001421 0.15 0.1421 0.5] Resize Logic
  (bind _output_get (Variables|Default|SetStartScale (.x (Variables|/Script/Engine.SceneComponent|GetRelativeScale3D (Variables|Character|GetMesh)))))
  (bind _newtrack_0 (Timeline|T_ScaleLerp PlayFromStart)
    (:Update
      (Transformation|SetActorScale3D (Math|Vector|MakeVector (Math|Float|Lerp _output_get TargetScale _newtrack_0) (Math|Float|Lerp _output_get TargetScale _newtrack_0) (Math|Float|Lerp _output_get TargetScale _newtrack_0))))))

(event Input|EnhancedActionEvents|EnhancedInputActionIA_TransformSmall
  (params (ActionValue :type Boolean) (ElapsedSeconds :type Float%20%28double-precision%29) (TriggeredSeconds :type Float%20%28double-precision%29) (InputAction :type Input%20Action%20Object%20Reference :default "/Game/Input/Actions/IA_TransformSmall.IA_TransformSmall"))
  ;[0.276 0.01914 0.002728 0.5] Input Ability Activation
  (:Started
    (Abilities|TryActivateAbilitybyClass (Variables|Default|GetAbilitySystemComponent) "/Game/GameplayAbilitySystem/Abilities/GA_Transform_Small.GA_Transform_Small_C" true)))

(event Input|EnhancedActionEvents|EnhancedInputActionIA_TransformBig
  (params (ActionValue :type Boolean) (ElapsedSeconds :type Float%20%28double-precision%29) (TriggeredSeconds :type Float%20%28double-precision%29) (InputAction :type Input%20Action%20Object%20Reference :default "/Game/Input/Actions/IA_TransformBig.IA_TransformBig"))
  ;[0.276 0.01914 0.002728 0.5] Input Ability Activation
  (:Started
    (Abilities|TryActivateAbilitybyClass (Variables|Default|GetAbilitySystemComponent) "/Game/GameplayAbilitySystem/Abilities/GA_Transform_Big.GA_Transform_Big_C" true)))

(event Input|EnhancedActionEvents|EnhancedInputActionIA_TransformNormal
  (params (ActionValue :type Boolean) (ElapsedSeconds :type Float%20%28double-precision%29) (TriggeredSeconds :type Float%20%28double-precision%29) (InputAction :type Input%20Action%20Object%20Reference :default "/Game/Input/Actions/IA_TransformNormal.IA_TransformNormal"))
  ;[0.276 0.01914 0.002728 0.5] Input Ability Activation
  (:Started
    (Abilities|TryActivateAbilitybyClass (Variables|Default|GetAbilitySystemComponent) "/Game/GameplayAbilitySystem/Abilities/GA_Transform_Normal.GA_Transform_Normal_C" true)))

(event Input|EnhancedActionEvents|EnhancedInputActionIA_Dash
  (params (ActionValue :type Boolean) (ElapsedSeconds :type Float%20%28double-precision%29) (TriggeredSeconds :type Float%20%28double-precision%29) (InputAction :type Input%20Action%20Object%20Reference :default "/Game/Input/Actions/IA_Dash.IA_Dash"))
  ;[0.276 0.01914 0.002728 0.5] Input Ability Activation
  (:Started
    (Abilities|TryActivateAbilitybyClass (Variables|Default|GetAbilitySystemComponent) "/Game/GameplayAbilitySystem/Abilities/ClassAbilities/GA_Pixie_Dash.GA_Pixie_Dash_C" true)))

(event Input|EnhancedActionEvents|EnhancedInputActionIA_Attk
  (params (ActionValue :type Boolean) (ElapsedSeconds :type Float%20%28double-precision%29) (TriggeredSeconds :type Float%20%28double-precision%29) (InputAction :type Input%20Action%20Object%20Reference :default "/Game/Input/Actions/IA_Attk.IA_Attk"))
  ;[0.276 0.01914 0.002728 0.5] Input Ability Activation
  (:Started
    (Abilities|TryActivateAbilitybyClass (Variables|Default|GetAbilitySystemComponent) "/Game/GameplayAbilitySystem/Abilities/GA_Melee.GA_Melee_C" true)))

(event EventBeginPlay
  ;[0.000769 0.15 0.00072 0.5] Begin Play
  (bind _asgi_game_instance (Utilities|Casting|CastToGI_GameInstance (Game|GetGameInstance)))
  (CallFunction|GrantDefaultAbilites&Effects)
  (switch Utilities|FlowControl|Switch|SwitchonE_CharacterClass (Variables|/Game/GI_GameInstance.GI_GameInstance_C|GetSelectedClass _asgi_game_instance)
    (:NewEnumerator0
      (CallFunction|GrantPixieAbilities))
    (:NewEnumerator1
      (CallFunction|GrantTitanAbilities))
    (:NewEnumerator2
      (CallFunction|GrantVersatileAbilites))))

(fn ConstructionScript)

(fn GrantVersatileAbilites
  (bind _returnvalue (Game|GetPlayerCharacter 0))
  (bind _returnvalue_2 (Ability|GetAbilitySystemComponent _returnvalue))
  (GameplayAbilities|GiveAbility _returnvalue_2 "/Game/GameplayAbilitySystem/Abilities/GA_Transform_Small.GA_Transform_Small_C" 0 -1)
  (GameplayAbilities|GiveAbility _returnvalue_2 "/Game/GameplayAbilitySystem/Abilities/GA_Transform_Big.GA_Transform_Big_C" 0 -1)
  (GameplayAbilities|GiveAbility _returnvalue_2 "/Game/GameplayAbilitySystem/Abilities/GA_Transform_Normal.GA_Transform_Normal_C" 0 -1)
  (GameplayEffects|ApplyGameplayEffectToSelf :self _returnvalue_2 :GameplayEffectClass "/Game/GameplayAbilitySystem/Effects/GrantClass/GE_Grant_Versatile.GE_Grant_Versatile_C"))

(fn GrantTitanAbilities
  (bind _returnvalue (Game|GetPlayerCharacter 0))
  (bind _returnvalue_2 (Ability|GetAbilitySystemComponent _returnvalue))
  (GameplayAbilities|GiveAbility _returnvalue_2 "/Game/GameplayAbilitySystem/Abilities/GA_Transform_Big.GA_Transform_Big_C" 0 -1)
  (GameplayAbilities|GiveAbility _returnvalue_2 "/Game/GameplayAbilitySystem/Abilities/GA_Transform_Normal.GA_Transform_Normal_C" 0 -1)
  (GameplayAbilities|GiveAbility _returnvalue_2 "/Game/GameplayAbilitySystem/Abilities/ClassAbilities/GA_Titan_Shockwave.GA_Titan_Shockwave_C" 0 -1)
  (GameplayEffects|ApplyGameplayEffectToSelf :self _returnvalue_2 :GameplayEffectClass "/Game/GameplayAbilitySystem/Effects/GrantClass/GE_Grant_Titan.GE_Grant_Titan_C"))

(fn GrantPixieAbilities
  (bind _returnvalue (Game|GetPlayerCharacter 0))
  (bind _returnvalue_2 (Ability|GetAbilitySystemComponent _returnvalue))
  (GameplayAbilities|GiveAbility _returnvalue_2 "/Game/GameplayAbilitySystem/Abilities/GA_Transform_Small.GA_Transform_Small_C" 0 -1)
  (GameplayAbilities|GiveAbility _returnvalue_2 "/Game/GameplayAbilitySystem/Abilities/GA_Transform_Normal.GA_Transform_Normal_C" 0 -1)
  (GameplayAbilities|GiveAbility _returnvalue_2 "/Game/GameplayAbilitySystem/Abilities/ClassAbilities/GA_Pixie_Dash.GA_Pixie_Dash_C" 0 -1)
  (GameplayEffects|ApplyGameplayEffectToSelf :self _returnvalue_2 :GameplayEffectClass "/Game/GameplayAbilitySystem/Effects/GrantClass/GE_Grant_Pixie.GE_Grant_Pixie_C"))

(fn GrantDefaultAbilites&Effects
  (bind _returnvalue (Game|GetPlayerCharacter 0))
  (bind _returnvalue_2 (Ability|GetAbilitySystemComponent _returnvalue))
  (GameplayEffects|ApplyGameplayEffectToSelf :self _returnvalue_2 :GameplayEffectClass "/Game/GameplayAbilitySystem/Effects/GE_InitStats.GE_InitStats_C" :Level 1.0)
  (GameplayEffects|ApplyGameplayEffectToSelf :self _returnvalue_2 :GameplayEffectClass "/Game/GameplayAbilitySystem/Effects/GE_Stamina_Regen.GE_Stamina_Regen_C")
  (GameplayAbilities|GiveAbility _returnvalue_2 "/Game/GameplayAbilitySystem/Abilities/GA_Melee.GA_Melee_C" 0 -1))