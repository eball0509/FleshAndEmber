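; Gameplay Ability that shrinks the player character into its small form, limited to owners with the Versatile class tag.
; On activation it commits only the cost, with no cooldown commit, then smoothly resizes BP_PlayerCharacter to 0.5.
; It applies GE_Form_Small and removes all stacks of GE_Form_Big, making the two forms mutually exclusive from this side, then ends immediately.
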(event Custom|CustomEvent_1
  (params (bWasCancelled :type Boolean))
  (Ability|EndAbility))

(event Ability|EventActivateAbility
  (if (GameplayTags|HasAnyTags (GameplayTags|MakeLiteralGameplayTagContainer "(GameplayTags=((TagName=\"Character.Class.Versatile\"),(TagName=\"Character.Class.Pixie\")))") (GameplayTags|GetOwnedGameplayTags (Ability|GetAbilitySystemComponentfromActorInfo) :!class /Script/GameplayTags.BlueprintGameplayTagLibrary))
    (Ability|CommitAbilityCost false)
    (bind _asbp_player_character (Utilities|Casting|CastToBP_PlayerCharacter (Ability|GetAvatarActorfromActorInfo)))
    (Variables|Default|SetASC (Ability|GetAbilitySystemComponent _asbp_player_character))
    (Default|MSmoothResize _asbp_player_character 0.5)
    (GameplayEffects|ApplyGameplayEffectToSelf :self (Variables|Default|GetASC) :GameplayEffectClass "/Game/GameplayAbilitySystem/Effects/States/GE_Form_Small.GE_Form_Small_C" :Level 1.0)
    (GameplayEffects|RemoveActiveGameplayEffectbySourceEffect (Variables|Default|GetASC) "/Game/GameplayAbilitySystem/Effects/States/GE_Form_Big.GE_Form_Big_C" 0 -1)
    (Ability|EndAbility)
    (else
      (Ability|EndAbility))))