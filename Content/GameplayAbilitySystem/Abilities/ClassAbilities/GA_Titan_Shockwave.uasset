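; GA_Titan_Shockwave is a Titan class Gameplay Ability that stuns enemies around the player.
; On activation it commits, then runs a sphere overlap at the player character's location for BP_Enemy pawns.
; Each enemy with a valid Ability System Component applies GE_Stun to itself; its attribute set is cached but unused.
; The ability ends after the loop or on a failed commit, but not if the avatar cast fails.
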(event Ability|EventActivateAbility
  (bind _returnvalue (Ability|CommitAbility))
  (if _returnvalue
    (bind _asbp_player_character (Utilities|Casting|CastToBP_PlayerCharacter (Ability|GetAvatarActorfromActorInfo)))
    (Variables|Default|SetPlayer%20REF _asbp_player_character)
    (bind _outactors (Collision|SphereOverlapActors (Transformation|GetActorLocation (Variables|Default|GetPlayer%20REF)) 1e+03 (Utilities|Array|MakeArray "ObjectTypeQuery3") "/Game/AI/BP_Enemy.BP_Enemy_C"))
    (for _array_element _outactors
      (Variables|Default|SetEnemyASC (Ability|GetAbilitySystemComponent _array_element))
      (Utilities|IsValid (Variables|Default|GetEnemyASC)
        (:Is%20Valid
          (bind _returnvalue_2 (GameplayAttributes|GetAttributeSet (Variables|Default|GetEnemyASC) "/Script/GAS_Test.DemoAttributes"))
          (Variables|Default|SetEnemy%20Attributes _returnvalue_2)
          (GameplayEffects|ApplyGameplayEffectToSelf :self (Variables|Default|GetEnemyASC) :GameplayEffectClass "/Game/GameplayAbilitySystem/Effects/GE_Stun.GE_Stun_C"))))
    (Ability|EndAbility)
    (else
      (Ability|EndAbility))))