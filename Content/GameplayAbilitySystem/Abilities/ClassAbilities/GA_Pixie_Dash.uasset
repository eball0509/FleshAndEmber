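; GA_Pixie_Dash is the Pixie class dash gameplay ability.
; On activation it commits cost and cooldown, then starts the dash cooldown display on the HUD reached through the first BP_WaveManager found in the world.
; It launches the avatar player character along its forward vector at DashSpeed, overriding horizontal velocity only, and ends immediately, or just ends if the commit fails.
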(event Ability|EventActivateAbility
  (bind _returnvalue (Ability|CommitAbility))
  (if _returnvalue
    (bind _outactors (Actor|GetAllActorsOfClass "/Game/BP_WaveManager.BP_WaveManager_C"))
    (Default|StartCooldownforTag (Variables|/Game/BP_WaveManager.BP_WaveManager_C|GetHud%20REF (Utilities|Array|Get(acopy) _outactors)) "(TagName=\"Cooldowns.Dash\")")
    (bind _asbp_player_character (Utilities|Casting|CastToBP_PlayerCharacter (Ability|GetAvatarActorfromActorInfo)))
    (Variables|Default|SetPlayer%20REF _asbp_player_character)
    (Character|LaunchCharacter (Variables|Default|GetPlayer%20REF) (* (Transformation|GetActorForwardVector (Variables|Default|GetPlayer%20REF)) (Variables|Default|GetDashSpeed)) true false)
    (Ability|EndAbility)
    (else
      (Ability|EndAbility))))