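; GA_Transform_Normal is a gameplay ability that returns a Titan-class player character to normal form.
; If the owner has the Titan class tag, it commits the ability cost, smoothly resizes the character to scale 1 and removes the Big and Small form gameplay effects.
; Without the tag it simply ends without doing anything else.
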(event Ability|EventActivateAbility
  (if (GameplayTags|HasAnyTags (GameplayTags|MakeLiteralGameplayTagContainer "(GameplayTags=((TagName=\"Character.Class.Titan\"),(TagName=\"Character.Class.Versatile\"),(TagName=\"Character.Class.Pixie\")))") (GameplayTags|GetOwnedGameplayTags (Ability|GetAbilitySystemComponentfromActorInfo) :!class /Script/GameplayTags.BlueprintGameplayTagLibrary))
    (Ability|CommitAbilityCost false)
    (bind _asbp_player_character (Utilities|Casting|CastToBP_PlayerCharacter (Ability|GetAvatarActorfromActorInfo)))
    (Variables|Default|SetASC (Ability|GetAbilitySystemComponent _asbp_player_character))
    (Default|MSmoothResize _asbp_player_character 1.0)
    (GameplayEffects|RemoveActiveGameplayEffectbySourceEffect (Variables|Default|GetASC) "/Game/GameplayAbilitySystem/Effects/States/GE_Form_Big.GE_Form_Big_C" 0 -1)
    (GameplayEffects|RemoveActiveGameplayEffectbySourceEffect (Variables|Default|GetASC) "/Game/GameplayAbilitySystem/Effects/States/GE_Form_Small.GE_Form_Small_C" 0 -1)
    (Ability|EndAbility)
    (else
      (Ability|EndAbility))))

(event Ability|EventOnEndAbility
  (params (bWasCancelled :type Boolean))
  (Ability|EndAbility))