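; Wave manager that spawns enemies in successive waves and creates the HUD showing wave number, enemies left and countdown.
; On BeginPlay it gathers all TargetPoints and starts the first wave from the Waves array.
; A looping timer spawns that wave's enemy class at random points until its count is reached.
; NotifyEnemyKilled tracks survivors and, once the wave is cleared, starts a timer-driven countdown to the next.
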(event Custom|AdvanceToNextWave
  (bind _waves (Variables|Arrays|GetWaves))
  (bind _output_get (Variables|Floats|SetCurrentWaveIndex (+ (Variables|Floats|GetCurrentWaveIndex) 1)))
  (Default|UpdateWaveInfo (Variables|Default|GetHud%20REF) (+ _output_get 1) (.EnemyCount (Utilities|Struct|BreakF_WaveData (Utilities|Array|Get(acopy) _waves (Variables|Floats|GetCurrentWaveIndex)))))
  (if (Utilities|Array|IsValidIndex _waves (Variables|Floats|GetCurrentWaveIndex))
    (Variables|Floats|SetEnemiesSpawnedThisWave 0)
    (Variables|Floats|SetEnemiesRemainingAlive (.EnemyCount (Utilities|Struct|BreakF_WaveData (Utilities|Array|Get(acopy) _waves (Variables|Floats|GetCurrentWaveIndex)))))
    (bind _returnvalue (Utilities|Time|SetTimerbyFunctionName 0 "SpawnSingleEnemy" (.SpawnInterval (Utilities|Struct|BreakF_WaveData (Utilities|Array|Get(acopy) _waves (Variables|Floats|GetCurrentWaveIndex)))) true))
    (Variables|TimerHandle|SetSpawnTimerHandle _returnvalue)))

(event Custom|StartCountdown
  (bind _returnvalue (Utilities|Time|SetTimerbyEvent (delegate Custom|TickCountdown) 0.1 true))
  (Variables|TimerHandle|SetWaveCountdownHandle _returnvalue))

(event Custom|TickCountdown
  (bind _output_get (Variables|Floats|SetTimeUntilNextWave (- (Variables|Floats|GetTimeUntilNextWave) 0.1)))
  (Default|UpdateWaveTimer (Variables|Default|GetHud%20REF) _output_get)
  (if (<= (Variables|Floats|GetTimeUntilNextWave) 0.0)
    (Utilities|Time|ClearandInvalidateTimerbyHandle (Variables|TimerHandle|GetWaveCountdownHandle))
    (CallFunction|AdvancetoNextWave)
    (Variables|Floats|SetTimeUntilNextWave 5.0)))

(event EventBeginPlay
  (bind _outactors (Actor|GetAllActorsOfClass "/Script/Engine.TargetPoint"))
  (Variables|Arrays|SetSpawnPoints _outactors)
  (bind _returnvalue (UserInterface|CreateWidget "/Game/UI/WBP_HUD.WBP_HUD_C" (Game|GetPlayerController 0)))
  (bind _output_get (Variables|Default|SetHud%20REF _returnvalue))
  (UserInterface|Viewport|AddtoViewport _output_get 0)
  (CallFunction|AdvancetoNextWave))

(fn ConstructionScript)

(fn SpawnSingleEnemy
  (bind _waves (Variables|Arrays|GetWaves))
  (bind _currentwaveindex (Variables|Floats|GetCurrentWaveIndex))
  (bind _output (Utilities|Array|Get(acopy) _waves _currentwaveindex))
  (bind (_enemyclass _enemycount) (Utilities|Struct|BreakF_WaveData _output))
  (if (< (Variables|Floats|GetEnemiesSpawnedThisWave) _enemycount)
    (Game|SpawnActorfromClass _enemyclass (Transformation|GetActorTransform (.OutItem (Utilities|Array|Random (Variables|Arrays|GetSpawnPoints)))) "AdjustIfPossibleButAlwaysSpawn" "MultiplyWithRoot" 0 0)
    (Variables|Floats|SetEnemiesSpawnedThisWave (+ (Variables|Floats|GetEnemiesSpawnedThisWave) 1))
    (if (>= (Variables|Floats|GetEnemiesSpawnedThisWave) _enemycount)
      (Utilities|Time|ClearandInvalidateTimerbyHandle (Variables|TimerHandle|GetSpawnTimerHandle)))
    (else
      (Utilities|Time|ClearandInvalidateTimerbyHandle (Variables|TimerHandle|GetSpawnTimerHandle)))))

(fn NotifyEnemyKilled
  (bind _output_get (Variables|Floats|SetEnemiesRemainingAlive (Math|Integer|Max(Integer) (- (Variables|Floats|GetEnemiesRemainingAlive) 1))))
  (Default|UpdateWaveInfo (Variables|Default|GetHud%20REF) (Variables|Floats|GetCurrentWaveIndex) _output_get)
  (if (and (<= (Variables|Floats|GetEnemiesRemainingAlive) 0) (>= (Variables|Floats|GetEnemiesSpawnedThisWave) (.enemycount (Utilities|Array|Get(acopy) (Variables|Arrays|GetWaves) (Variables|Floats|GetCurrentWaveIndex)))))
    (CallFunction|StartCountdown)))

(fn RemoveHUD
  (Widget|RemovefromParent (Variables|Default|GetHud%20REF)))